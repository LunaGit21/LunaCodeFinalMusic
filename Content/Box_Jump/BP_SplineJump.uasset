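; BP_SplineJump is an actor that plots and displays an arced jump path from the player to a hit point.
; HitResult passes the target and normal to SpawnFun, which range-checks distance, builds a three-point spline with a distance-scaled apex and downward landing tangent, and orients HitPoint to the surface.
; The spline is shown via the "show splines" console command.
; Timeline logic to move the player along it exists but is disconnected.
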(event EventBeginPlay
  (bind _returnvalue (PlayerController|LocalPlayerSubsystems|GetEnhancedInputLocalPlayerSubsystem))
  (Utilities|IsValid _returnvalue
    (:Is%20Valid
      (Input|AddMappingContext _returnvalue "/Game/FirstPerson/Input/IMC_Default.IMC_Default" 0 "(bIgnoreAllPressedKeysUntilRelease=True,bForceImmediately=False,bNotifyUserSettings=False)"))))

(event EventTick
  (params (DeltaSeconds :type Float%20%28single-precision%29)))

(event EventHitResult
  (params (OutputHit :type Hit%20Result%20Structure) (Targethit :type Vector :default "0, 0, 0") (TargetNormal :type Vector :default "0, 0, 0"))
  (CallFunction|SpawnFun Targethit TargetNormal))

(event Collision|EventActorBeginOverlap
  (params (OtherActor :type Actor%20Object%20Reference)))

(event Input|KeyboardEvents|2
  (params (Key :type Key%20Structure)))

(fn ConstructionScript)

(fn SpawnFun
  (params (JumpTo :type Vector) (JumpLandNormal :type Vector))
  (bind _output_get (Variables|Default|SetJumpTo JumpTo))
  (Variables|Default|SetJumpLandNormal JumpLandNormal)
  (bind _output_get_2 (Variables|Default|SetJumpDistance (Math|Vector|Distance(Vector) _output_get (Transformation|GetWorldLocation (Variables|/Script/Engine.Character|GetCapsuleComponent (Game|GetPlayerCharacter 0))))))
  (Variables|Default|SetReadyToJump (Math|Float|InRange(Float) _output_get_2 1.0 1.5e+04))
  (bind _output_get_3 (Variables|Default|SetJumpFrom (Transformation|GetWorldLocation (Variables|/Script/Engine.Character|GetCapsuleComponent (Game|GetPlayerCharacter 0)))))
  (Spline|SetSplinePoints (Variables|Default|GetSplineForJump) (Utilities|Array|MakeArray _output_get_3 (+ (* (+ _output_get_3 (Variables|Default|GetJumpTo)) 0.5) (Math|Vector|MakeVector 0.0 0.0 (* 0.5 (Variables|Default|GetJumpDistance)))) (Variables|Default|GetJumpTo)) "World" true)
  (Spline|SetTangentatSplinePoint (Variables|Default|GetSplineForJump) 2 (* "0.000000,0.000000,-1.000000" (Math|Float|Clamp(Float) (Variables|Default|GetJumpDistance) 0.0 2e+03)) "World" true)
  (Transformation|SetWorldLocationAndRotation (Variables|Default|GetHitPoint) (Variables|Default|GetJumpTo) (Math|Conversions|RotationFromXVector (Variables|Default|GetJumpLandNormal)) false false)
  (Rendering|SetVisibility (Variables|Default|GetSplineForJump) true true)
  (Development|ExecuteConsoleCommand "show splines" 0)
  (Utilities|Casting|CastToBP_FirstPersonCharacter (Game|GetPlayerCharacter 0)))